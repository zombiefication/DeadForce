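; Base player weapon Blueprint that fires projectiles with recoil and a heat-based overheat mechanic.
; Shots spawn at the muzzle, aimed at a camera trace point, and receive damage, crit and impact settings.
; Each shot adds heat; at maximum, firing locks until a looping timer cools it to zero while not firing.
; Timelines smooth displayed heat and drive recoil; Tick repeats an alarm while the equipped weapon is overheated.
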(event `self.ReceiveBeginPlay`
  (bind _heattimeline (`self.HeatTimeline`))
  (`self.BeginReduceHeat`)
  (`TimelineComponent.SetPlayRate` _heattimeline (/ (`TimelineComponent.GetTimelineLength` _heattimeline) (`self.FiringRate`))))

(event `self.ReceiveTick`
  (params (DeltaSeconds :type "Float (single-precision)"))
  (`self.OverheatAlarm`))

(event `FireWeapon`
  ;[1 1 1] Fire Weapon
  (if (`self.WeaponOverheated`)
    (`self.StopFireWeapon`)
    (else
      (`SkeletalMeshComponent.PlayAnimation` (`self.WeaponMesh`) (`self.WeaponFireAnimation`) false)
      (bind _projectilespawninfo (`self.CalaculateShootInfo`))
      (bind _returnvalue (`|SpawnActorFromClass` (`self.ProjectileClass`) _projectilespawninfo "AlwaysSpawn" "OverrideRootScale" null (`self.GetInstigator`)))
      (`/Game/Weapons/Projectiles/BaseProjectile_BP.SetDamageInfo` _returnvalue (`self.DamageMin`) (`self.DamageMax`) (`self.CritChance`) (`self.ImpactForce`))
      (`self.FireHeatBuildup`)
      (`self.Recoil`))))

(event `StopFireWeapon`)

(event `Recoil`
  (bind _returnvalue (`GameplayStatics.GetPlayerController` 0))
  ;[1 1 1] Recoil
  (bind (_direction _recoilamount) (`Timeline|RecoilTimeline` :!via `PlayFromStart`)
    (:`Update`
      (`PlayerController.AddPitchInput` _returnvalue (`KismetMathLibrary.Lerp` 0.0 (* (`self.VerticalRecoil`) -1.0) _recoilamount))
      (`PlayerController.AddYawInput` _returnvalue (`KismetMathLibrary.Lerp` 0.0 (`self.HorizontalRecoil`) _recoilamount)))))

(event `BeginReduceHeat`
  ;[1 1 1] Begin Reduce Heat
  (bind _returnvalue (`KismetSystemLibrary.K2_SetTimerDelegate` (delegate `ReduceHeat`) (`self.FiringRate`) true))
  (set `self.ReduceHeatTimer` _returnvalue))

(event `ReduceHeat`
  ;[1 1 1] Reduce Heat
  (if (and (not (`self.IsFiring`)) (> (`self.HeatCurrent`) 0.0))
    (bind _output_get (set `self.HeatPrevious` (`self.HeatCurrent`)))
    (`|ExecutionSequence`
      (:`then_0`
        (bind _returnvalue (- _output_get (`self.HeatReductionRate`)))
        (if (<= _returnvalue 0.0)
          (set `self.HeatCurrent` 0.0)
          (set `self.WeaponOverheated` false)
          (else
            (set `self.HeatCurrent` _returnvalue))))
      (:`then_1`
        (`self.PerformUpdateHeat`)))))

(event `PerformUpdateHeat`
  ;[1 1 1] Update Heat
  (bind (_direction _heat) (`Timeline|HeatTimeline` :!via `PlayFromStart`)
    (:`Update`
      (set `self.HeatDisplayed` (/ (`KismetMathLibrary.Lerp` (`self.HeatPrevious`) (`self.HeatCurrent`) _heat) (`self.HeatMax`))))))

(fn `CalaculateShootInfo`
  (returns (ProjectileSpawnInfo :type "Transform Structure"))
  (bind _playercamera (`self.PlayerCamera`))
  (bind _returnvalue (`SceneComponent.K2_GetComponentLocation` _playercamera))
  (bind _returnvalue_2 (`SceneComponent.GetSocketLocation` (`self.WeaponMesh`) "Muzzle"))
  (bind (_outhit _returnvalue_3) (`KismetSystemLibrary.LineTraceSingle` _returnvalue (+ _returnvalue (* (`SceneComponent.GetForwardVector` _playercamera) 10000.0)) "TraceTypeQuery3"))
  (if _returnvalue_3
    (bind (_bblockinghit _binitialoverlap _time _location _impactpoint _normal _impactnormal _physmat _hitactor _hitcomponent _hitbonename _hititem _tracestart _traceend) (`GameplayStatics.BreakHitResult` _outhit))
    (return (`KismetMathLibrary.MakeTransform` _returnvalue_2 (`KismetMathLibrary.FindLookAtRotation` _returnvalue_2 _impactpoint)))
    (else
      (return (`KismetMathLibrary.MakeTransform` _returnvalue_2 (`KismetMathLibrary.FindLookAtRotation` _returnvalue_2 _traceend))))))

(fn `FireHeatBuildup`
  (bind _returnvalue (+ (`self.HeatCurrent`) (`self.HeatBuildUpRate`)))
  (`|ExecutionSequence`
    (:`then_0`
      (set `self.HeatPrevious` (`self.HeatCurrent`)))
    (:`then_1`
      (if (>= _returnvalue (`self.HeatMax`))
        (set `self.HeatCurrent` (`self.HeatMax`))
        (set `self.WeaponOverheated` true)
        (else
          (set `self.HeatCurrent` _returnvalue))))
    (:`then_2`
      (`self.PerformUpdateHeat`))))

(fn `SetCamera`
  (params (Camera :type "CameraComponent Object Reference"))
  (set `self.PlayerCamera` Camera))

(fn `UserConstructionScript`)