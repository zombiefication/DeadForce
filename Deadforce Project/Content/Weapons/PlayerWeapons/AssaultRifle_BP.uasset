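; AssaultRifle_BP is a player weapon Blueprint that adds automatic fire to its parent weapon's firing behavior.
; FireWeapon sets IsFiring, fires immediately, then starts a looping timer at FiringRate that calls AutomaticFire.
; AutomaticFire delegates each shot to the parent FireWeapon while IsFiring is true.
; StopFireWeapon clears the flag and invalidates the timer to end firing.
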(event `self.FireWeapon`
  (set `self.IsFiring` true)
  (`self.AutomaticFire`)
  (bind _returnvalue (`KismetSystemLibrary.K2_SetTimerDelegate` (delegate `AutomaticFire`) (`self.FiringRate`) true))
  (set `self.AutomaticFireTimer` _returnvalue))

(event `AutomaticFire`
  (if (`self.IsFiring`)
    (`parent.FireWeapon`)))

(event `self.StopFireWeapon`
  (set `self.IsFiring` false)
  (`KismetSystemLibrary.K2_ClearAndInvalidateTimerHandle` (`self.AutomaticFireTimer`)))

(fn `UserConstructionScript`
  (`parent.UserConstructionScript`))